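; CheckpointResetBox is a trigger volume that sends the first-person player back to a checkpoint on overlap.
; When the collider is entered by the FirstPersonCharacter, it searches all Checkpoint actors for the one whose number matches its own CheckpointNumber and moves the player to that actor's location.
; If HurtsPlayerToReset is set, it also deals DamageAmount to the player, then stops the search.
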(event OnComponentBeginOverlap(Collider)
  (params (OverlappedComponent :type Primitive%20Component%20Object%20Reference) (OtherActor :type Actor%20Object%20Reference) (OtherComp :type Primitive%20Component%20Object%20Reference) (OtherBodyIndex :type Integer) (bFromSweep :type Boolean) (SweepResult :type Hit%20Result%20Structure%20%28by%20ref%29))
  (bind _asfirst_person_character (Utilities|Casting|CastToFirstPersonCharacter OtherActor))
  (bind _outactors (Actor|GetAllActorsOfClass "/Game/Blueprints/Checkpoint.Checkpoint_C"))
  (bind _array_element (Utilities|Array|ForEachLoopwithBreak _outactors :!label _label)
    (:LoopBody
      (if (== (Variables|Default|GetCheckpointNumber) (Variables|/Game/Blueprints/Checkpoint.Checkpoint_C|GetCheckpointNumber _array_element))
        (Transformation|SetActorLocation _asfirst_person_character (Transformation|GetActorLocation _array_element) false false)
        (if (Variables|Default|GetHurts%20Player%20To%20Reset)
          (Default|ReceiveDamage _asfirst_person_character (Variables|Default|GetDamageAmount))
          (goto _label Break)
          (else
            (goto _label Break)))))))

(event EventBeginPlay)

(event Collision|EventActorBeginOverlap
  (params (OtherActor :type Actor%20Object%20Reference)))

(event EventTick
  (params (DeltaSeconds :type Float%20%28single-precision%29)))

(fn ConstructionScript)