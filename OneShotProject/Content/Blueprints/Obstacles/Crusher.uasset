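; Crusher is an obstacle actor that deals lethal damage to the player on contact.
; Its Hit event passes the other actor to CheckPlayerHit, which ignores other Crushers and casts the rest to FirstPersonCharacter.
; A matching character receives damage equal to its current Health.
; The Blueprint holds no movement logic, and its BeginPlay, overlap and Tick events are disabled stubs.
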(event EventBeginPlay
  (|CallParentFunction) ; This node is disabled and will not be called.\nDrag off pins to build functionality.
)

(event Collision|EventActorBeginOverlap
  (params (OtherActor :type Actor%20Object%20Reference))
  (|CallParentFunction OtherActor) ; This node is disabled and will not be called.\nDrag off pins to build functionality.
)

(event EventTick
  (params (DeltaSeconds :type Float%20%28single-precision%29))
  (|CallParentFunction DeltaSeconds) ; This node is disabled and will not be called.\nDrag off pins to build functionality.
)

(event Collision|EventHit
  (params (MyComp :type Primitive%20Component%20Object%20Reference) (Other :type Actor%20Object%20Reference) (OtherComp :type Primitive%20Component%20Object%20Reference) (bSelfMoved :type Boolean) (HitLocation :type Vector :default "0, 0, 0") (HitNormal :type Vector :default "0, 0, 0") (NormalImpulse :type Vector :default "0, 0, 0") (Hit :type Hit%20Result%20Structure%20%28by%20ref%29))
  (CallFunction|CheckPlayerHit Other)
  (Utilities|IsValid OtherComp))

(fn ConstructionScript
  (|CallParentFunction))

(fn CheckPlayerHit
  (params (Object :type Actor%20Object%20Reference))
  (Utilities|Casting|CastToCrusher Object
    (:CastFailed
      (bind _asfirst_person_character (Utilities|Casting|CastToFirstPersonCharacter Object))
      (Default|ReceiveDamage _asfirst_person_character (Variables|/Game/FirstPersonBP/Blueprints/FirstPersonCharacter.FirstPersonCharacter_C|GetHealth _asfirst_person_character)))))