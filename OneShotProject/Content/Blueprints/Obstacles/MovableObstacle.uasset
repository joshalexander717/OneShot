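; MovableObstacle is an obstacle that shuttles a component back and forth between its construction-time location and that point plus MovementAmount.
; After an initial StartDelay, Tick moves it by the Speed vector each frame, reversing via the MovingToEnd flag.
; Endpoints are detected within a 1-unit tolerance, where pauses are counted in ticks, so both motion and waits depend on frame rate.
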(event EventBeginPlay)

(event Collision|EventActorBeginOverlap
  (params (OtherActor :type Actor%20Object%20Reference)))

(event EventTick
  (params (DeltaSeconds :type Float%20%28single-precision%29))
  (bind _movingcomponent (Variables|Default|GetMovingComponent))
  (bind _returnvalue (Transformation|GetWorldLocation _movingcomponent))
  (if (Variables|Default|GetHasDelayed)
    _
    (else
      (Utilities|FlowControl|Delay (Variables|Default|GetStartDelay))
      (Variables|Default|SetHasDelayed true)))
  (if (Math|Vector|Equal(Vector) (Variables|Default|GetStartPos) _returnvalue 1.0)
    (if (> (Variables|Default|GetTicksSinceStartPause) (Variables|Default|GetPauseStart))
      (Variables|Default|SetMovingToEnd true)
      (Variables|Default|SetTicksSinceEndPause 0)
      (CallFunction|MovetoEnd :!label _label)
      (else
        (Math|Integer|IncrementInt (Variables|Default|GetTicksSinceStartPause))))
    (elif (Math|Vector|Equal(Vector) _returnvalue (Variables|Default|GetEndPos) 1.0)
      (if (> (Variables|Default|GetTicksSinceEndPause) (Variables|Default|GetPauseEnd))
        (Variables|Default|SetMovingToEnd false)
        (Variables|Default|SetTicksSinceStartPause 0)
        (CallFunction|MovetoStart :!label _label_2)
        (else
          (Math|Integer|IncrementInt (Variables|Default|GetTicksSinceEndPause))))
      (elif (Variables|Default|GetMovingToEnd)
        (goto _label)
        (else
          (goto _label_2))))))

(fn ConstructionScript
  (bind _movingcomponent (Variables|Default|GetMovingComponent))
  (bind _returnvalue (Transformation|GetWorldLocation _movingcomponent))
  (Variables|Default|SetStartPos _returnvalue)
  (Variables|Default|SetEndPos (+ _returnvalue (Variables|Default|GetMovementAmount))))

(fn MovetoEnd
  (bind _movingcomponent (Variables|Default|GetMovingComponent))
  (Transformation|SetWorldLocation _movingcomponent (+ (Transformation|GetWorldLocation _movingcomponent) (Variables|Default|GetSpeed)) false false))

(fn MovetoStart
  (bind _movingcomponent (Variables|Default|GetMovingComponent))
  (Transformation|SetWorldLocation _movingcomponent (+ (Transformation|GetWorldLocation _movingcomponent) (* (Variables|Default|GetSpeed) -1)) false false))