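; Crusher trap obstacle whose spikes move back and forth on a timed cycle and damage the first-person character.
; After a start delay, a FlipFlop alternates playing and reversing a timeline that drives the spikes' relative location, with a separate wait before each stroke and each finish retriggering it.
; Box overlap deals damage at most once per forward stroke, as a flag blocks hits during the return phase.
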(event OnComponentBeginOverlap(Box)
  (params (OverlappedComponent :type Primitive%20Component%20Object%20Reference) (OtherActor :type Actor%20Object%20Reference) (OtherComp :type Primitive%20Component%20Object%20Reference) (OtherBodyIndex :type Integer) (bFromSweep :type Boolean) (SweepResult :type Hit%20Result%20Structure%20%28by%20ref%29))
  (if (not (Variables|Default|GetHasHurtPlayer))
    (bind _asfirst_person_character (Utilities|Casting|CastToFirstPersonCharacter OtherActor))
    (Default|ReceiveDamage _asfirst_person_character (Variables|Default|GetDamageAmount))
    (Variables|Default|SetHasHurtPlayer true)))

(event EventBeginPlay
  (Utilities|FlowControl|Delay (Variables|Default|GetStart%20Delay))
  (Variables|Default|SetStartPos (Transformation|GetWorldLocation (Variables|Default|GetSpikes)))
  (Utilities|FlowControl|FlipFlop :!label _label
    (:A
      (Utilities|FlowControl|Delay (Variables|Default|GetTimeUp))
      (Variables|Default|SetHasHurtPlayer false)
      (bind _spiketrack (Timeline|Timeline_0 PlayFromStart)
        (:Update
          (Transformation|SetRelativeLocation (Variables|Default|GetSpikes) (Math|Vector|MakeVector 0.0 0.0 _spiketrack) false false))
        (:Finished
          (goto _label))))
    (:B
      (Variables|Default|SetHasHurtPlayer true)
      (Utilities|FlowControl|Delay (Variables|Default|GetTimeDown))
      (Timeline|Timeline_0 ReverseFromEnd))))

(event Collision|EventActorBeginOverlap
  (params (OtherActor :type Actor%20Object%20Reference)))

(event EventTick
  (params (DeltaSeconds :type Float%20%28single-precision%29)))

(fn ConstructionScript)