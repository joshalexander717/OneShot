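; TextPopupBox is a trigger actor that shows a one-time text popup when the FirstPersonCharacter overlaps its Collider.
; On that overlap it creates a PopupTextWidget with its text, pause and tutorial-tip settings, adds it to the viewport and plays its fade-in.
; It optionally pauses the game, then sets HasAppeared so the popup does not show again.
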(event OnComponentBeginOverlap(Collider)
  (params (OverlappedComponent :type Primitive%20Component%20Object%20Reference) (OtherActor :type Actor%20Object%20Reference) (OtherComp :type Primitive%20Component%20Object%20Reference) (OtherBodyIndex :type Integer) (bFromSweep :type Boolean) (SweepResult :type Hit%20Result%20Structure%20%28by%20ref%29))
  (if (not (Variables|Default|GetHasAppeared))
    (Utilities|Casting|CastToFirstPersonCharacter OtherActor)
    (bind _returnvalue (UserInterface|CreateWidget "/Game/UI/PopupTextWidget.PopupTextWidget_C" 0 (Variables|Default|GetPopup%20Text) (Variables|Default|GetPauses%20Game) (Variables|Default|GetTutorialTip) (Variables|Default|GetTutorialTipTime)))
    (bind _output_get (Variables|Default|SetPopupWidget _returnvalue))
    (UserInterface|Viewport|AddtoViewport _output_get 0)
    (UserInterface|Animation|PlayAnimation _output_get (Variables|/Game/UI/PopupTextWidget.PopupTextWidget_C|GetFadeIn _output_get) 0.0 1 "Forward" 1.0 false)
    (if (Variables|Default|GetPauses%20Game)
      (Game|SetGamePaused true))
    (Variables|Default|SetHasAppeared true)))

(event EventBeginPlay)

(event Collision|EventActorBeginOverlap
  (params (OtherActor :type Actor%20Object%20Reference)))

(event EventTick
  (params (DeltaSeconds :type Float%20%28single-precision%29)))

(fn ConstructionScript)