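; Pickup actor that gives the overlapping FirstPersonCharacter a power-up type for a set lifetime.
; On overlap it sets the character's current power-up, starts its countdown, destroys itself and prints the display name.
; A restarting timeline drives the intended mesh bob by nudging it from its current height each update, so offsets accumulate.
; Tick spins the whole actor around yaw at a frame-rate-independent rate.
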(event EventBeginPlay
  (bind _staticmesh (Variables|Default|GetStaticMesh))
  (bind _returnvalue (Transformation|GetWorldLocation _staticmesh))
  (bind (_x _y _z) (Math|Vector|BreakVector _returnvalue))
  ;[1 1 1] Move static mesh up and down
  (bind (_direction _floattrack) (Timeline|MovementTimeline Play)
    (:Update
      (bind _output_get (Variables|Default|SetMoveLocation (Math|Vector|Lerp(Vector) _returnvalue (Math|Vector|MakeVector _x _y (+ _z 0.5)) _floattrack)))
      (Transformation|SetWorldLocation _staticmesh _output_get true false))
    (:Finished
      (switch Utilities|FlowControl|Switch|SwitchonETimelineDirection _direction
        (:Forward
          (Timeline|MovementTimeline PlayFromStart))
        (:Backward
          (Timeline|MovementTimeline ReverseFromEnd))))))

(event Collision|EventActorBeginOverlap
  (params (OtherActor :type Actor%20Object%20Reference))
  ;[1 1 1] Add powerup to player
  (bind _asfirst_person_character (Utilities|Casting|CastToFirstPersonCharacter OtherActor))
  (Variables|/Game/FirstPersonBP/Blueprints/FirstPersonCharacter.FirstPersonCharacter_C|SetCurrentPowerUp _asfirst_person_character (Variables|Default|GetPowerUpType))
  (Default|PowerUpCountdown _asfirst_person_character (Variables|Default|GetPowerUpLifetime))
  (Actor|DestroyActor)
  (Development|PrintString (Utilities|String|Append "Picked up power up: " (Variables|Default|GetDisplayName))))

(event EventTick
  (params (DeltaSeconds :type Float%20%28single-precision%29))
  ;[1 1 1] Rotate static mesh
  (Transformation|AddActorLocalRotation (Math|Rotator|MakeRotator 0.0 0.0 (* (Variables|Default|GetRotationRate) DeltaSeconds)) false false))

(fn ConstructionScript)