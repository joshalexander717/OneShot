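; Test actor Blueprint that sends an HTTP GET to a remote profile endpoint on BeginPlay using the VaRest plugin.
; It builds a URL-encoded request carrying hardcoded username and password fields, binds completion and failure callbacks, then applies the URL.
; The callbacks only print the response code and body, or a failure message, to screen.
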(event Custom|RequestComplete
  (params (Request :type Va%20Rest%20Request%20JSON%20Object%20Reference))
  (bind _returnvalue (Class|VaRestRequestJSON|GetResponseContentasString Request true))
  (Development|PrintString (Utilities|String|ToString(Integer) (Class|VaRestRequestJSON|GetResponseCode Request)))
  (Development|PrintString _returnvalue))

(event Custom|RequestFail
  (params (Request :type Va%20Rest%20Request%20JSON%20Object%20Reference))
  (Development|PrintString "Request Failed"))

(event EventBeginPlay
  (Development|PrintString "Hello")
  (bind _returnvalue (Class|VaRestSubsystem|ConstructVaRestRequestExt (|VaRestSubsystem) "GET" "x_www_form_urlencoded_url"))
  (bind _output_get (Variables|Default|SetMyRequest _returnvalue))
  (EventDispatchers|BindEventtoOnRequestComplete _output_get (delegate Custom|RequestComplete))
  (EventDispatchers|BindEventtoOnRequestFail _output_get (delegate Custom|RequestFail))
  (Class|VaRestJsonObject|SetStringField (Class|VaRestRequestJSON|GetRequestObject (Variables|Default|GetMyRequest)) "username" "altajack")
  (Class|VaRestJsonObject|SetStringField (Class|VaRestRequestJSON|GetRequestObject (Variables|Default|GetMyRequest)) "password" "password")
  (Class|VaRestRequestJSON|ApplyURL _output_get "http://ec2-54-86-216-199.compute-1.amazonaws.com:8080/profile"))

(event Collision|EventActorBeginOverlap
  (params (OtherActor :type Actor%20Object%20Reference)))

(event EventTick
  (params (DeltaSeconds :type Float%20%28single-precision%29)))

(fn ConstructionScript)