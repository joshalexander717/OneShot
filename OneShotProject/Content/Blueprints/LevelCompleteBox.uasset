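; Level exit trigger box that ends the level when the player overlaps it, either immediately or only once no BaseEnemy remains, depending on the level type.
; Shortly after BeginPlay it also seeds the HUD's slow-mo meter with the level's amount.
; LevelComplete stops the timer, scores three configurable star challenges from time, enemy and player-flag checks, then freezes movement and shows the completion screen with UI-only input.
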(event OnComponentBeginOverlap(CollisionBox)
  (params (OverlappedComponent :type Primitive%20Component%20Object%20Reference) (OtherActor :type Actor%20Object%20Reference) (OtherComp :type Primitive%20Component%20Object%20Reference) (OtherBodyIndex :type Integer) (bFromSweep :type Boolean) (SweepResult :type Hit%20Result%20Structure%20%28by%20ref%29))
  (Utilities|Casting|CastToFirstPersonCharacter OtherActor
    (:then
      (switch Utilities|FlowControl|Switch|SwitchonLevelType (Variables|Default|GetType%20Of%20Level)
        (:NewEnumerator0
          (bind _outactors (Actor|GetAllActorsOfClass "/Game/Blueprints/Enemies/BaseEnemy.BaseEnemy_C"))
          (if (not (> (Utilities|Array|Length _outactors) 0))
            (CallFunction|LevelComplete :!label _label)))
        (:NewEnumerator1
          (goto _label))))
    (:CastFailed
      (Development|PrintString "CAST FAILED"))))

(event EventBeginPlay
  (Utilities|FlowControl|Delay 0.1)
  (bind _asfirst_person_character (Utilities|Casting|CastToFirstPersonCharacter (Game|Player|GetPlayerPawn 0)))
  (bind _output_get (Variables|/Game/UI/HUD.HUD_C|SetMaxSlowmo (Variables|/Game/FirstPersonBP/Blueprints/FirstPersonCharacter.FirstPersonCharacter_C|GetPlayerHUD _asfirst_person_character) (Variables|Default|GetLevel%20Slowmo%20Amount)))
  (Variables|/Game/UI/HUD.HUD_C|SetCurrentSlowmo (Variables|/Game/FirstPersonBP/Blueprints/FirstPersonCharacter.FirstPersonCharacter_C|GetPlayerHUD _asfirst_person_character) _output_get))

(event Collision|EventActorBeginOverlap
  (params (OtherActor :type Actor%20Object%20Reference)))

(event EventTick
  (params (DeltaSeconds :type Float%20%28single-precision%29)))

(fn ConstructionScript)

(fn LevelComplete
  (bind _returnvalue (Game|Player|GetPlayerPawn 0))
  (bind _returnvalue_2 (Game|GetPlayerController 0))
  (bind _returnvalue_3 (Game|Player|GetPlayerPawn 0))
  (bind _timetobeat (Variables|Default|GetTimeToBeat))
  (bind _asfirst_person_character (Utilities|Casting|CastToFirstPersonCharacter _returnvalue_3))
  (bind _asfirst_person_character_2 (Utilities|Casting|CastToFirstPersonCharacter _returnvalue))
  (bind _hasreloaded (Variables|/Game/FirstPersonBP/Blueprints/FirstPersonCharacter.FirstPersonCharacter_C|GetHasReloaded _asfirst_person_character_2))
  (bind _charactermovement (Variables|/Script/Engine.Character|GetCharacterMovement _asfirst_person_character))
  (bind _playerhud (Variables|/Game/FirstPersonBP/Blueprints/FirstPersonCharacter.FirstPersonCharacter_C|GetPlayerHUD _asfirst_person_character_2))
  (bind _hasmissed (Variables|/Game/FirstPersonBP/Blueprints/FirstPersonCharacter.FirstPersonCharacter_C|GetHasMissed _asfirst_person_character_2))
  (bind _hastakendamage (Variables|/Game/FirstPersonBP/Blueprints/FirstPersonCharacter.FirstPersonCharacter_C|GetHasTakenDamage _asfirst_person_character_2))
  (bind _returnvalue_4 (not _hastakendamage))
  (bind _returnvalue_5 (not _hasreloaded))
  (bind _returnvalue_6 (not _hasmissed))
  (bind _timer (Variables|/Game/UI/HUD.HUD_C|GetTimer _playerhud))
  (bind _elapsedtime (Variables|/Game/UI/Timer.Timer_C|GetElapsedTime _timer))
  (bind _returnvalue_7 (> _timetobeat _elapsedtime))
  (Variables|/Game/UI/Timer.Timer_C|SetStopped _timer true)
  (bind _returnvalue_8 (Actor|GetActorOfClass "/Game/Blueprints/Enemies/BaseEnemy.BaseEnemy_C"))
  (Variables|Default|SethasKilledAllEnemies (not (Utilities|IsValid _returnvalue_8)))
  (Variables|Default|SetStar1Obtained (Utilities|Select :Index (Variables|Default|GetStar1) :NewEnumerator0 _returnvalue_7 :NewEnumerator1 _returnvalue_5 :NewEnumerator2 _returnvalue_4 :NewEnumerator4 (Variables|Default|GethasKilledAllEnemies) :NewEnumerator5 _returnvalue_6))
  (Variables|Default|SetStar2Obtained (Utilities|Select :Index (Variables|Default|GetStar2) :NewEnumerator0 _returnvalue_7 :NewEnumerator1 _returnvalue_5 :NewEnumerator2 _returnvalue_4 :NewEnumerator4 (Variables|Default|GethasKilledAllEnemies) :NewEnumerator5 _returnvalue_6))
  (Variables|Default|SetStar3Obtained (Utilities|Select :Index (Variables|Default|GetStar3) :NewEnumerator0 _returnvalue_7 :NewEnumerator1 _returnvalue_5 :NewEnumerator2 _returnvalue_4 :NewEnumerator4 (Variables|Default|GethasKilledAllEnemies) :NewEnumerator5 _returnvalue_6))
  (Variables|/Game/FirstPersonBP/Blueprints/FirstPersonCharacter.FirstPersonCharacter_C|SetLevelComplete _asfirst_person_character true)
  (Variables|/Script/Engine.MovementComponent|SetVelocity _charactermovement "0, 0, 0")
  (Pawn|Components|CharacterMovement|DisableMovement _charactermovement)
  (bind _returnvalue_9 (UserInterface|CreateWidget "/Game/UI/LevelCompleteScreen.LevelCompleteScreen_C" 0 (Variables|Default|GetStar1Obtained) (Variables|Default|GetStar2Obtained) (Variables|Default|GetStar3Obtained)))
  (UserInterface|Viewport|AddtoViewport _returnvalue_9 0)
  (Input|SetInputModeUIOnly _returnvalue_2 _returnvalue_9 "DoNotLock")
  (Variables|/Script/Engine.PlayerController|SetbShowMouseCursor _returnvalue_2 true))