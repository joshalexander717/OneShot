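; Pickup actor that grants the first-person character health, a thrust reset or slowmo charge, chosen by PickupType.
; On overlap it applies the effect, clamping health and the HUD-held slowmo value, then destroys itself and prints its name.
; Tick spins the actor in yaw, while a replaying timeline moves the Plane mesh on Z, meant as a bob but lerping from its current location each update.
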(event EventBeginPlay
  (bind _plane (Variables|Default|GetPlane))
  (bind _returnvalue (Transformation|GetWorldLocation _plane))
  (bind (_x _y _z) (Math|Vector|BreakVector _returnvalue))
  ;[1 1 1] Move static mesh up and down
  (bind (_direction _floattrack) (Timeline|MovementTimeline Play)
    (:Update
      (bind _output_get (Variables|Default|SetMoveLocation (Math|Vector|Lerp(Vector) _returnvalue (Math|Vector|MakeVector _x _y (+ _z 0.5)) _floattrack)))
      (Transformation|SetWorldLocation _plane _output_get true false))
    (:Finished
      (switch Utilities|FlowControl|Switch|SwitchonETimelineDirection _direction
        (:Forward
          (Timeline|MovementTimeline PlayFromStart))
        (:Backward
          (Timeline|MovementTimeline ReverseFromEnd))))))

(event Collision|EventActorBeginOverlap
  (params (OtherActor :type Actor%20Object%20Reference))
  ;[1 1 1] Add powerup to player
  (bind _asfirst_person_character (Utilities|Casting|CastToFirstPersonCharacter OtherActor))
  (switch Utilities|FlowControl|Switch|SwitchonPickups_Enum (Variables|Default|GetPickupType)
    (:NewEnumerator0
      (Variables|/Game/FirstPersonBP/Blueprints/FirstPersonCharacter.FirstPersonCharacter_C|SetHealth _asfirst_person_character (Math|Integer|Clamp(Integer) (+ (Variables|/Game/FirstPersonBP/Blueprints/FirstPersonCharacter.FirstPersonCharacter_C|GetHealth _asfirst_person_character) (Variables|Default|GetHealthGainAmount)) 0 (Variables|/Game/FirstPersonBP/Blueprints/FirstPersonCharacter.FirstPersonCharacter_C|GetMax%20Health _asfirst_person_character))))
    (:NewEnumerator1
      (Variables|/Game/FirstPersonBP/Blueprints/FirstPersonCharacter.FirstPersonCharacter_C|SetCurrentThrustTime _asfirst_person_character 0.0)
      (Variables|/Game/FirstPersonBP/Blueprints/FirstPersonCharacter.FirstPersonCharacter_C|SetFirstThrust _asfirst_person_character true))
    (:NewEnumerator2
      (Variables|/Game/UI/HUD.HUD_C|SetCurrentSlowmo (Variables|/Game/FirstPersonBP/Blueprints/FirstPersonCharacter.FirstPersonCharacter_C|GetPlayerHUD _asfirst_person_character) (Math|Float|Clamp(Float) (+ (Variables|/Game/UI/HUD.HUD_C|GetCurrentSlowmo (Variables|/Game/FirstPersonBP/Blueprints/FirstPersonCharacter.FirstPersonCharacter_C|GetPlayerHUD _asfirst_person_character)) (Variables|Default|GetSlowmoGainAmount)) 0.0 (Variables|/Game/UI/HUD.HUD_C|GetMaxSlowmo (Variables|/Game/FirstPersonBP/Blueprints/FirstPersonCharacter.FirstPersonCharacter_C|GetPlayerHUD _asfirst_person_character))))))
  (Actor|DestroyActor)
  (Development|PrintString (Utilities|String|Append "Pickup: " (Variables|Default|GetDisplayName))))

(event EventTick
  (params (DeltaSeconds :type Float%20%28single-precision%29))
  ;[1 1 1] Rotate static mesh
  (Transformation|AddActorLocalRotation (Math|Rotator|MakeRotator 0.0 0.0 (* (Variables|Default|GetRotationRate) DeltaSeconds)) false false))

(fn ConstructionScript)