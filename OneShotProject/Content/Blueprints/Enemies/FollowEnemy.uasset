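; FollowEnemy is an enemy that chases the first-person player and damages them on contact.
; When Pawn Sensing sees a FirstPersonCharacter, AI Move To follows it, using DetectionRadius as the acceptance radius.
; Hit events run CheckPlayerHit, which ignores BaseEnemy actors and applies a small fixed damage to the player through ReceiveDamage.
; BeginPlay, overlap and Tick are disabled stubs, and the OtherComp validity check leads nowhere.
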(event OnSeePawn(PawnSensing)
  (params (Pawn :type Pawn%20Object%20Reference))
  (bind _asfirst_person_character (Utilities|Casting|CastToFirstPersonCharacter Pawn))
  (AI|AIMoveTo self "0, 0, 0" _asfirst_person_character (Variables|Default|GetDetectionRadius) false))

(event EventBeginPlay
  (|CallParentFunction) ; This node is disabled and will not be called.\nDrag off pins to build functionality.
)

(event Collision|EventActorBeginOverlap
  (params (OtherActor :type Actor%20Object%20Reference))
  (|CallParentFunction OtherActor) ; This node is disabled and will not be called.\nDrag off pins to build functionality.
)

(event EventTick
  (params (DeltaSeconds :type Float%20%28single-precision%29))
  (|CallParentFunction DeltaSeconds) ; This node is disabled and will not be called.\nDrag off pins to build functionality.
)

(event Collision|EventHit
  (params (MyComp :type Primitive%20Component%20Object%20Reference) (Other :type Actor%20Object%20Reference) (OtherComp :type Primitive%20Component%20Object%20Reference) (bSelfMoved :type Boolean) (HitLocation :type Vector :default "0, 0, 0") (HitNormal :type Vector :default "0, 0, 0") (NormalImpulse :type Vector :default "0, 0, 0") (Hit :type Hit%20Result%20Structure%20%28by%20ref%29))
  ;[1 1 1] Damage
  (CallFunction|CheckPlayerHit Other)
  (Utilities|IsValid OtherComp))

(fn ConstructionScript
  (|CallParentFunction))

(fn CheckPlayerHit
  (params (Object :type Actor%20Object%20Reference))
  (Utilities|Casting|CastToBaseEnemy Object
    (:CastFailed
      (bind _asfirst_person_character (Utilities|Casting|CastToFirstPersonCharacter Object))
      (Default|ReceiveDamage _asfirst_person_character 2))))