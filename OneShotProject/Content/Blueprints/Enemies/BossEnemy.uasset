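; Boss enemy Blueprint that detects the player within a sphere, faces them and fires projectiles.
; While the player is nearby, a repeating camera-channel line trace sets SeesPlayer, which drives per-tick yaw rotation and starts a looping countdown for moving or shooting.
; Shoot briefly changes State while spawning an EnemyProjectile aimed at the player.
; RunToNewLocation and Teleporting are empty here, and the death dissolve-style material effect is unconnected.
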(event OnComponentBeginOverlap(Sphere)
  (params (OverlappedComponent :type Primitive%20Component%20Object%20Reference) (OtherActor :type Actor%20Object%20Reference) (OtherComp :type Primitive%20Component%20Object%20Reference) (OtherBodyIndex :type Integer) (bFromSweep :type Boolean) (SweepResult :type Hit%20Result%20Structure%20%28by%20ref%29))
  (Utilities|Casting|CastToFirstPersonCharacter OtherActor)
  (Variables|Default|SetPlayerNearby true)
  (CallFunction|LookforPlayerEvent))

(event OnComponentEndOverlap(Sphere)
  (params (OverlappedComponent :type Primitive%20Component%20Object%20Reference) (OtherActor :type Actor%20Object%20Reference) (OtherComp :type Primitive%20Component%20Object%20Reference) (OtherBodyIndex :type Integer))
  (Utilities|Casting|CastToFirstPersonCharacter OtherActor)
  (Variables|Default|SetPlayerNearby false))

(event Custom|RunToNewLocation)

(event Custom|LookForPlayerEvent
  (if (Variables|Default|GetPlayerNearby)
    (bind _outhit (Collision|LineTraceByChannel (Transformation|GetActorLocation) (Transformation|GetActorLocation (Game|Player|GetPlayerPawn 0)) "TraceTypeQuery2" false 0 "None"))
    (Utilities|Casting|CastToFirstPersonCharacter (.HitActor (Collision|BreakHitResult _outhit))
      (:then
        (if (Variables|Default|GetSeesPlayer)
          (Variables|Default|SetSeesPlayer true)
          (else
            (Variables|Default|SetSeesPlayer true)
            (CallFunction|SeesPlayerEvent))))
      (:CastFailed
        (Variables|Default|SetSeesPlayer false)))
    (Utilities|FlowControl|Delay (* (Utilities|Time|GetWorldDeltaSeconds) 3e+01))
    (CallFunction|LookforPlayerEvent)))

(event Custom|SeesPlayerEvent
  (bind _state (Variables|Default|GetState))
  (if (Variables|Default|GetSeesPlayer)
    (if (or (Utilities|Enum|Equal(Enum) _state "NewEnumerator1") (Utilities|Enum|Equal(Enum) _state "NewEnumerator2"))
      _
      (elif (<= (Variables|Default|GetCurrentTimeUntilMove) 0.0)
        (Variables|Default|SetCurrentTimeUntilMove (Variables|Default|GetTimeUntilMove))
        (CallFunction|RuntoNewLocation)
        (else
          (Variables|Default|SetCurrentTimeUntilMove (- (Variables|Default|GetCurrentTimeUntilMove) 0.1))
          (if (<= (Variables|Default|GetCurrentTImeUntilShoot) 0.0)
            (Variables|Default|SetCurrentTImeUntilShoot (Variables|Default|GetTimeUntilShoot))
            (CallFunction|Shoot)
            (else
              (Variables|Default|SetCurrentTImeUntilShoot (- (Variables|Default|GetCurrentTImeUntilShoot) 0.1)))))))
    (Utilities|FlowControl|Delay 0.2)
    (CallFunction|SeesPlayerEvent)))

(event Custom|Shoot
  (Variables|Default|SetState "NewEnumerator2")
  (bind _returnvalue (Game|SpawnActorfromClass "/Game/Blueprints/Enemies/EnemyProjectile.EnemyProjectile_C" (Math|Transform|MakeTransform (Transformation|GetWorldLocation (Variables|Default|GetShootPoint)) (Math|Rotator|FindLookatRotation (Transformation|GetActorLocation) (Transformation|GetActorLocation (Game|Player|GetPlayerPawn 0)))) "Undefined" 0 0 0))
  (Variables|/Game/Blueprints/Enemies/EnemyProjectile.EnemyProjectile_C|SetParentEnemy _returnvalue self)
  (Utilities|FlowControl|Delay 0.2)
  (Variables|Default|SetState "NewEnumerator0"))

(event EventBeginPlay
  (|CallParentFunction))

(event Collision|EventActorBeginOverlap
  (params (OtherActor :type Actor%20Object%20Reference))
  (|CallParentFunction OtherActor))

(event EventTick
  (params (DeltaSeconds :type Float%20%28single-precision%29))
  (|CallParentFunction DeltaSeconds)
  (if (Variables|Default|GetSeesPlayer)
    (Transformation|SetActorRotation (Math|Rotator|MakeRotator 0.0 0.0 (.Yaw (Math|Rotator|BreakRotator (Math|Rotator|FindLookatRotation (Transformation|GetActorLocation) (Transformation|GetActorLocation (Game|Player|GetPlayerPawn 0)))))))))

(fn ConstructionScript
  (|CallParentFunction))

(fn Teleporting)

(fn SeesPlayerFunc
  (|CallParentFunction))