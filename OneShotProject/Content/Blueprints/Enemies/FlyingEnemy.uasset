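; Flying enemy that faces a visible player, fires projectiles and teleports around its spawn point.
; A sphere overlap starts a repeating line-of-sight trace, which starts a countdown loop choosing between teleporting and delayed shots, both blocked while stunned.
; Teleporting uses a timeline to scale the capsule, relocates it mid-way if a trace is clear, then reverses the scale.
; The trace and destination roll separate random points.
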(event OnComponentBeginOverlap(Sphere)
  (params (OverlappedComponent :type Primitive%20Component%20Object%20Reference) (OtherActor :type Actor%20Object%20Reference) (OtherComp :type Primitive%20Component%20Object%20Reference) (OtherBodyIndex :type Integer) (bFromSweep :type Boolean) (SweepResult :type Hit%20Result%20Structure%20%28by%20ref%29))
  (Utilities|Casting|CastToFirstPersonCharacter OtherActor)
  (Variables|Default|SetPlayerNearby true)
  (CallFunction|LookforPlayerEvent))

(event OnComponentEndOverlap(Sphere)
  (params (OverlappedComponent :type Primitive%20Component%20Object%20Reference) (OtherActor :type Actor%20Object%20Reference) (OtherComp :type Primitive%20Component%20Object%20Reference) (OtherBodyIndex :type Integer))
  (Utilities|Casting|CastToFirstPersonCharacter OtherActor)
  (Variables|Default|SetPlayerNearby false))

(event Custom|Teleport
  (bind _returnvalue (Math|Random|RandomUnitVector))
  (bind _returnvalue_2 (Transformation|GetActorLocation))
  (bind _initial_location (Variables|Default|GetInitial%20Location))
  (bind _returnvalue_3 (* _returnvalue 5e+02))
  (bind _returnvalue_4 (+ _initial_location _returnvalue_3))
  (if (not (Variables|Default|GetIsStunned))
    (Variables|Default|SetFinishedTeleporting false)
    (Variables|Default|SetState "NewEnumerator1")
    (bind _scale (Timeline|TeleportTimeline Play)
      (:Update
        (Transformation|SetWorldScale3D (Variables|Default|GetCapsuleComponent) (Math|Vector|MakeVector _scale _scale _scale)))
      (:Finished
        (if (Variables|Default|GetFinishedTeleporting)
          (Variables|Default|SetState "NewEnumerator0")
          (else
            (Utilities|FlowControl|Delay 0.1)
            (Variables|Default|SetFinishedTeleporting true)
            (bind (_outhit _returnvalue_5) (Collision|LineTraceByChannel _returnvalue_2 _returnvalue_4 "TraceTypeQuery1" false 0 "None"))
            (Transformation|SetActorLocation (Math|Vector|SelectVector _returnvalue_2 _returnvalue_4 _returnvalue_5) false false)
            (Timeline|TeleportTimeline ReverseFromEnd)))))))

(event Custom|LookForPlayerEvent
  (if (Variables|Default|GetPlayerNearby)
    (bind _outhit (Collision|LineTraceByChannel (Transformation|GetActorLocation) (Transformation|GetActorLocation (Game|Player|GetPlayerPawn 0)) "TraceTypeQuery2" false 0 "None"))
    (Utilities|Casting|CastToFirstPersonCharacter (.HitActor (Collision|BreakHitResult _outhit))
      (:then
        (if (Variables|Default|GetSeesPlayer)
          (Variables|Default|SetSeesPlayer true)
          (else
            (Variables|Default|SetSeesPlayer true)
            (CallFunction|SeesPlayerEvent))))
      (:CastFailed
        (Variables|Default|SetSeesPlayer false)))
    (Utilities|FlowControl|Delay (* (Utilities|Time|GetWorldDeltaSeconds) 3e+01))
    (CallFunction|LookforPlayerEvent)))

(event Custom|SeesPlayerEvent
  (bind _state (Variables|Default|GetState))
  (if (Variables|Default|GetSeesPlayer)
    (if (or (Utilities|Enum|Equal(Enum) _state "NewEnumerator1") (Utilities|Enum|Equal(Enum) _state "NewEnumerator2"))
      _
      (elif (<= (Variables|Default|GetCurrentTimeUntilTeleport) 0.0)
        (Variables|Default|SetCurrentTimeUntilTeleport (Variables|Default|GetTimeUntilTeleport))
        (CallFunction|Teleport)
        (else
          (Variables|Default|SetCurrentTimeUntilTeleport (- (Variables|Default|GetCurrentTimeUntilTeleport) 0.1))
          (if (<= (Variables|Default|GetCurrentTImeUntilShoot) 0.0)
            (Variables|Default|SetCurrentTImeUntilShoot (Variables|Default|GetTimeUntilShoot))
            (CallFunction|Shoot)
            (else
              (Variables|Default|SetCurrentTImeUntilShoot (- (Variables|Default|GetCurrentTImeUntilShoot) 0.1)))))))
    (Utilities|FlowControl|Delay 0.2)
    (CallFunction|SeesPlayerEvent)))

(event Custom|Shoot
  (if (not (Variables|Default|GetIsStunned))
    (Variables|Default|SetState "NewEnumerator2")
    (Utilities|FlowControl|Delay 2.5)
    (Game|SpawnActorfromClass "/Game/Blueprints/Enemies/EnemyProjectile.EnemyProjectile_C" (Math|Transform|MakeTransform (Transformation|GetWorldLocation (Variables|Default|GetShootPoint)) (Transformation|GetActorRotation)) "Undefined" 0 self 0)
    (Utilities|FlowControl|Delay 1.0)
    (Variables|Default|SetState "NewEnumerator0")))

(event EventBeginPlay
  (|CallParentFunction)
  (Variables|Default|SetInitial%20Location (Transformation|GetActorLocation)))

(event Collision|EventActorBeginOverlap
  (params (OtherActor :type Actor%20Object%20Reference))
  (|CallParentFunction OtherActor))

(event EventTick
  (params (DeltaSeconds :type Float%20%28single-precision%29))
  (|CallParentFunction DeltaSeconds)
  (if (Variables|Default|GetSeesPlayer)
    (Transformation|SetActorRotation (Math|Rotator|FindLookatRotation (Transformation|GetActorLocation) (Transformation|GetActorLocation (Game|Player|GetPlayerPawn 0))))))

(fn ConstructionScript
  (|CallParentFunction))

(fn Teleporting)

(fn SeesPlayerFunc
  (|CallParentFunction))