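; Jackal enemy AI that chases the player and makes melee attacks.
; A proximity sphere starts a repeating line-trace sight check, which moves it toward the player's location, while Tick turns it to face a spotted player.
; An attack trigger loops timed attacks that set its state and, after a short wind-up, deal damage if the player overlaps the damage volume.
; Being stunned blocks movement orders and new attacks.
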(event OnComponentBeginOverlap(Sphere)
  (params (OverlappedComponent :type Primitive%20Component%20Object%20Reference) (OtherActor :type Actor%20Object%20Reference) (OtherComp :type Primitive%20Component%20Object%20Reference) (OtherBodyIndex :type Integer) (bFromSweep :type Boolean) (SweepResult :type Hit%20Result%20Structure%20%28by%20ref%29))
  ;[1 1 1] BaseAI Code
  (Utilities|Casting|CastToFirstPersonCharacter OtherActor)
  (Variables|Default|SetPlayerNearby true)
  (CallFunction|LookforPlayerEvent))

(event OnComponentEndOverlap(Sphere)
  (params (OverlappedComponent :type Primitive%20Component%20Object%20Reference) (OtherActor :type Actor%20Object%20Reference) (OtherComp :type Primitive%20Component%20Object%20Reference) (OtherBodyIndex :type Integer))
  ;[1 1 1] BaseAI Code
  (Utilities|Casting|CastToFirstPersonCharacter OtherActor)
  (Variables|Default|SetPlayerNearby false))

(event OnComponentBeginOverlap(PlayerAttackDetection)
  (params (OverlappedComponent :type Primitive%20Component%20Object%20Reference) (OtherActor :type Actor%20Object%20Reference) (OtherComp :type Primitive%20Component%20Object%20Reference) (OtherBodyIndex :type Integer) (bFromSweep :type Boolean) (SweepResult :type Hit%20Result%20Structure%20%28by%20ref%29))
  ;[1 0.5642 0.5642] Jackal Functions
  (Utilities|Casting|CastToFirstPersonCharacter OtherActor)
  (Variables|Default|SetLookingForAttacks true)
  (if (Variables|Default|GetLookingForAttacks) :!label _label
    (CallFunction|Attack)
    (Utilities|FlowControl|Delay 2.0)
    (goto _label)))

(event OnComponentBeginOverlap(PlayerDamageDetection)
  (params (OverlappedComponent :type Primitive%20Component%20Object%20Reference) (OtherActor :type Actor%20Object%20Reference) (OtherComp :type Primitive%20Component%20Object%20Reference) (OtherBodyIndex :type Integer) (bFromSweep :type Boolean) (SweepResult :type Hit%20Result%20Structure%20%28by%20ref%29))
  ;[1 0.5642 0.5642] Jackal Functions
  (Utilities|Casting|CastToFirstPersonCharacter OtherActor)
  (Variables|Default|SetJackalDamageCollidingWithPlayer true))

(event OnComponentEndOverlap(PlayerDamageDetection)
  (params (OverlappedComponent :type Primitive%20Component%20Object%20Reference) (OtherActor :type Actor%20Object%20Reference) (OtherComp :type Primitive%20Component%20Object%20Reference) (OtherBodyIndex :type Integer))
  ;[1 0.5642 0.5642] Jackal Functions
  (Utilities|Casting|CastToFirstPersonCharacter OtherActor)
  (Variables|Default|SetJackalDamageCollidingWithPlayer false))

(event OnComponentEndOverlap(PlayerAttackDetection)
  (params (OverlappedComponent :type Primitive%20Component%20Object%20Reference) (OtherActor :type Actor%20Object%20Reference) (OtherComp :type Primitive%20Component%20Object%20Reference) (OtherBodyIndex :type Integer))
  ;[1 0.5642 0.5642] Jackal Functions
  (Utilities|Casting|CastToFirstPersonCharacter OtherActor)
  (Variables|Default|SetLookingForAttacks false))

(event Custom|RunToNewLocation
  ;[1 1 1] BaseAI Code
)

(event Custom|LookForPlayerEvent
  ;[1 1 1] BaseAI Code
  (if (Variables|Default|GetPlayerNearby)
    (bind _outhit (Collision|LineTraceByChannel (Transformation|GetActorLocation) (Transformation|GetActorLocation (Game|Player|GetPlayerPawn 0)) "TraceTypeQuery2" false 0 "None"))
    (Utilities|Casting|CastToFirstPersonCharacter (.HitActor (Collision|BreakHitResult _outhit))
      (:then
        (Variables|Default|SetSeesPlayer true)
        (CallFunction|SeesPlayerEvent))
      (:CastFailed
        (Variables|Default|SetSeesPlayer false)))
    (Utilities|FlowControl|Delay (* (Utilities|Time|GetWorldDeltaSeconds) 3e+01))
    (CallFunction|LookforPlayerEvent)))

(event Custom|SeesPlayerEvent
  ;[1 0.5642 0.5642] Jackal Functions
  (if (Utilities|Enum|Equal(Enum) (Variables|Default|GetState) "NewEnumerator2")
    _
    (else
      (Variables|Default|SetState "NewEnumerator1")))
  (if (not (Variables|Default|GetIsStunned))
    (AI|AIMoveTo self (Transformation|GetActorLocation (Game|Player|GetPlayerPawn 0)) 0 1.0 false)))

(event Custom|Attack
  ;[1 0.5642 0.5642] Jackal Functions
  (if (not (Variables|Default|GetIsStunned))
    (Variables|Default|SetState "NewEnumerator2")
    (Utilities|FlowControl|Delay 0.2)
    (if (Variables|Default|GetJackalDamageCollidingWithPlayer)
      (Default|ReceiveDamage (.AsFirst%20Person%20Character (Utilities|Casting|CastToFirstPersonCharacter (Game|Player|GetPlayerPawn 0))) (Variables|Default|GetDamage)))
    (Utilities|FlowControl|Delay 0.2)
    (Variables|Default|SetState "NewEnumerator1")))

(event EventBeginPlay
  ;[1 1 1] BaseAI Code
  (|CallParentFunction))

(event Collision|EventActorBeginOverlap
  (params (OtherActor :type Actor%20Object%20Reference))
  ;[1 1 1] BaseAI Code
  (|CallParentFunction OtherActor))

(event EventTick
  (params (DeltaSeconds :type Float%20%28single-precision%29))
  ;[1 1 1] BaseAI Code
  (|CallParentFunction DeltaSeconds)
  (if (Variables|Default|GetSeesPlayer)
    (Transformation|SetActorRotation (Math|Rotator|MakeRotator 0.0 0.0 (.Yaw (Math|Rotator|BreakRotator (Math|Rotator|FindLookatRotation (Transformation|GetActorLocation) (Transformation|GetActorLocation (Game|Player|GetPlayerPawn 0)))))))))

(fn ConstructionScript
  (|CallParentFunction))

(fn Teleporting)

(fn SeesPlayerFunc
  (|CallParentFunction))