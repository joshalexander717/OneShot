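; RangeEnemy is an enemy that turns to face the first-person player it sees and fires projectiles at them.
; PawnSensing triggers the look-at rotation and spawns an EnemyProjectile from the capsule, unless the enemy is stunned.
; The fire rate is counted in Tick frames rather than seconds, so it varies with frame rate, and the construction script pre-fills the counter so the first shot is ready immediately.
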(event OnSeePawn(PawnSensing)
  (params (Pawn :type Pawn%20Object%20Reference))
  (bind _capsulecomponent (Variables|Default|GetCapsuleComponent))
  (bind _returnvalue (Transformation|GetWorldLocation _capsulecomponent))
  (if (not (Variables|Default|GetIsStunned))
    (bind _asfirst_person_character (Utilities|Casting|CastToFirstPersonCharacter Pawn))
    (Transformation|SetActorRotation (Math|Rotator|FindLookatRotation _returnvalue (Transformation|GetWorldLocation (Variables|/Script/Engine.Character|GetCapsuleComponent _asfirst_person_character))))
    (if (== (Variables|Default|GetTicksBetweenShots) (Variables|Default|GetTicksSinceLastShot))
      (Game|SpawnActorfromClass "/Game/Blueprints/Enemies/EnemyProjectile.EnemyProjectile_C" (Math|Transform|MakeTransform _returnvalue (Transformation|GetActorRotation) "1,1,1") "Undefined" 0 0)
      (Variables|Default|SetTicksSinceLastShot 0))))

(event EventBeginPlay
  (|CallParentFunction) ; This node is disabled and will not be called.\nDrag off pins to build functionality.
)

(event Collision|EventActorBeginOverlap
  (params (OtherActor :type Actor%20Object%20Reference))
  (|CallParentFunction OtherActor) ; This node is disabled and will not be called.\nDrag off pins to build functionality.
)

(event EventTick
  (params (DeltaSeconds :type Float%20%28single-precision%29))
  (bind _tickssincelastshot (Variables|Default|GetTicksSinceLastShot))
  (|CallParentFunction DeltaSeconds)
  (if (> (Variables|Default|GetTicksBetweenShots) _tickssincelastshot)
    (Math|Integer|IncrementInt _tickssincelastshot)))

(fn ConstructionScript
  (|CallParentFunction)
  (Variables|Default|SetTicksSinceLastShot (Variables|Default|GetTicksBetweenShots)))