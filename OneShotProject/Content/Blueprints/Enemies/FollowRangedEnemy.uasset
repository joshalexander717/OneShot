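; Ranged enemy that follows the first-person player and shoots projectiles at them.
; When PawnSensing sees the player, it starts an AI move toward them using DetectionRadius as acceptance radius, firing immediately without waiting for arrival if the cooldown has elapsed.
; Shots spawn at the capsule's location with the actor's rotation.
; The cooldown counts Tick frames, so fire rate is frame-rate dependent; construction applies WalkSpeed to movement.
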(event OnSeePawn(PawnSensing)
  (params (Pawn :type Pawn%20Object%20Reference))
  (bind _asfirst_person_character (Utilities|Casting|CastToFirstPersonCharacter Pawn))
  (AI|AIMoveTo self "0, 0, 0" _asfirst_person_character (Variables|Default|GetDetectionRadius) false
    (:then
      (if (== (Variables|Default|GetTicksBetweenShots) (Variables|Default|GetTicksSinceLastShot))
        (Game|SpawnActorfromClass "/Game/Blueprints/Enemies/EnemyProjectile.EnemyProjectile_C" (Math|Transform|MakeTransform (Transformation|GetWorldLocation (Variables|Default|GetCapsuleComponent)) (Transformation|GetActorRotation) "1,1,1") "Undefined" 0 0)
        (Variables|Default|SetTicksSinceLastShot 0)))))

(event EventBeginPlay
  (|CallParentFunction) ; This node is disabled and will not be called.\nDrag off pins to build functionality.
)

(event Collision|EventActorBeginOverlap
  (params (OtherActor :type Actor%20Object%20Reference))
  (|CallParentFunction OtherActor) ; This node is disabled and will not be called.\nDrag off pins to build functionality.
)

(event EventTick
  (params (DeltaSeconds :type Float%20%28single-precision%29))
  (bind _tickssincelastshot (Variables|Default|GetTicksSinceLastShot))
  (|CallParentFunction DeltaSeconds)
  (if (> (Variables|Default|GetTicksBetweenShots) _tickssincelastshot)
    (Math|Integer|IncrementInt _tickssincelastshot)))

(fn ConstructionScript
  (|CallParentFunction)
  (Variables|/Script/Engine.CharacterMovementComponent|SetMaxWalkSpeed (Variables|Character|GetCharacterMovement) (Variables|Default|GetWalkSpeed)))